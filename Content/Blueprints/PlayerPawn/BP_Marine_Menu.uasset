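; BP_Marine_Menu is a Marine player pawn Blueprint, apparently a menu variant, holding twin-stick style aim helpers and an alive check.
; Mouse velocity is input delta over frame time; above a deadzone, its angle becomes a yaw that control rotation interpolates toward.
; Thumbstick input above its own deadzone sets control rotation yaw directly, without smoothing.
; No event graph here calls these functions, and the construction script is empty.
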(fn ConstructionScript)

(fn UpdateMouseAim
  (if (MouseInput|IsMouseAboveDeadzone)
    (Pawn|SetControlRotation (Game|GetPlayerController 0) (MouseInput|GetMouseAimDirection))))

(fn IsThumbstickAboveDeadzone
  (return (> (Math|Vector2D|Vector2DLength (Math|Vector2D|MakeVector2D (Input|AxisValues|GetThumbstickAimRight) (Input|AxisValues|GetThumbstickAimUp))) (Variables|ThumbstickInput|GetThumbstickDeadzone))))

(fn GetMouseVelocity
  (bind _returnvalue (Game|GetPlayerController 0))
  (bind (_deltax _deltay) (Class|PlayerController|GetInputMouseDelta _returnvalue))
  (return (/ (Math|Vector2D|MakeVector2D _deltax _deltay) (Utilities|Time|GetWorldDeltaSeconds))))

(fn IsMouseAboveDeadzone
  (return (> (Math|Vector2D|Vector2DLength (MouseInput|GetMouseVelocity)) (Variables|MouseInput|GetMouseDeadzone))))

(fn GetMouseAimDirection
  (bind _returnvalue (MouseInput|GetMouseVelocity))
  (return (Math|Interpolation|RInterpTo (Pawn|GetControlRotation (Game|GetPlayerController 0) :!class /Script/Engine.Controller) (Math|Rotator|MakeRotator 0.0 0.0 (Class|KismetMathLibrary|DegAtan2 (.x _returnvalue) (.y _returnvalue))) (Utilities|Time|GetWorldDeltaSeconds) (Variables|MouseInput|GetMouse%20Smoothing%20Strength))))

(fn UpdateJoystickAim
  (if (ThumbstickInput|IsThumbstickAboveDeadzone)
    (Pawn|SetControlRotation (Game|GetPlayerController 0) (Math|Rotator|MakeRotator 0.0 0.0 (Class|KismetMathLibrary|DegAtan2 (Input|AxisValues|GetThumbstickAimRight) (Input|AxisValues|GetThumbstickAimUp))))))

(fn IsAlive
  (return (not (Variables|Default|GetDead))))