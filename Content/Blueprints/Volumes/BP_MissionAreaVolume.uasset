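; BP_MissionAreaVolume is a mission boundary volume that damages the player for leaving the playable area.
; Overlap begin and end events toggle OutsideMissionArea on BP_Marine; re-entry clears the damage timer.
; Exit waits briefly, then starts a looping timer that applies LeavingAreaDamage to player character 0.
; Re-entering during that delay does not cancel it, so the timer still starts.
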(event Collision|EventActorBeginOverlap
  (params (OtherActor :type Actor%20Object%20Reference))
  ;[1 1 1] Player Enter Mission Area
  (bind _asbp_marine (Utilities|Casting|CastToBP_Marine OtherActor))
  (Variables|/Game/Blueprints/PlayerPawn/BP_Marine.BP_Marine_C|SetOutside%20Mission%20Area _asbp_marine false)
  (Utilities|Time|ClearTimerbyFunctionName 0 "Reduce Player Health"))

(event Collision|EventActorEndOverlap
  (params (OtherActor :type Actor%20Object%20Reference))
  ;[1 1 1] Player leaves Mission Area
  (bind _asbp_marine (Utilities|Casting|CastToBP_Marine OtherActor))
  (Variables|/Game/Blueprints/PlayerPawn/BP_Marine.BP_Marine_C|SetOutside%20Mission%20Area _asbp_marine true)
  (Utilities|FlowControl|Delay 1.0)
  (Utilities|Time|SetTimerbyFunctionName 0 "Reduce Player Health" 1.5 true))

(fn ConstructionScript)

(fn ReducePlayerHealth
  (Game|Damage|ApplyDamage (Game|GetPlayerCharacter 0) (Variables|Default|GetLeaving%20Area%20Damage) 0 0))